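; BP_Bump is a grenade-like explosive actor that knocks the player character away and breaks BP_Destructible actors.
; GrenadelLancee runs a timed fuse, then sets Explosion, spawns an emitter and self-destroys, while Dynamo triggers the launch immediately.
; Tick faces the player and, if exploding within range, launches them once along the look-at direction, factoring in their velocity.
; Destructibles ending overlap with Sphere1 during an explosion get AutoDestruction.
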(event `self.ReceiveBeginPlay`
  (`|ExecutionSequence`
    (:`then_0`
      (bind _asbp_third_person_character (cast `/Game/Blueprints/BP_ThirdPersonCharacter` (`GameplayStatics.GetPlayerCharacter` 0)))
      (set `self.As BP Third Person Character` _asbp_third_person_character))))

(event `Grenadel Lancee`
  (set `self.Explosion` false)
  (`KismetSystemLibrary.Delay` 2.5)
  (set `self.Explosion` true)
  (if (`self.Explosion`)
    (`GameplayStatics.SpawnEmitterAtLocation` null (`self.K2_GetActorLocation`) (struct) (10.0 10.0 10.0))
    (`KismetSystemLibrary.Delay` 0.5)
    (`self.K2_DestroyActor` :!label _label)))

(event `self.ReceiveTick`
  (params (DeltaSeconds :type "Float (single-precision)"))
  (bind _returnvalue (`self.K2_GetActorLocation`))
  (bind _returnvalue_2 (`KismetMathLibrary.FindLookAtRotation` _returnvalue (`self.K2_GetActorLocation` (`self.As BP Third Person Character`))))
  (`|ExecutionSequence`
    (:`then_0`
      (`self.K2_SetActorRotation` _returnvalue_2))
    (:`then_1`
      (if (`self.Explosion`)
        (if (`self.Close`)
          (`/Engine/EditorBlueprintResources/StandardMacros.DoOnce` false
            (:`Completed`
              (`Character.LaunchCharacter` (`self.As BP Third Person Character`) (* (`KismetMathLibrary.RotateAngleAxis` (`KismetMathLibrary.Conv_RotatorToVector` _returnvalue_2) 0.0 _returnvalue) (+ (2000.0 2000.0 500.0) (`self.GetVelocity` (`self.As BP Third Person Character`)))) false false :!label _label_2)
              (goto _label))))))
    (:`then_2`
      (if (<= (`KismetMathLibrary.Vector_Distance` (`self.K2_GetActorLocation` (`self.As BP Third Person Character`)) (`self.K2_GetActorLocation`)) 200.0)
        (set `self.Close` true)
        (else
          (set `self.Close` false))))))

(event `Dynamo`
  (set `self.Explosion` true)
  (goto _label_2))

(event `Colliding`
  (if (`self.Explosion`)
    (`/Game/Trash/BP_Destructible.Auto Destruction` (stale `self.Sphere1.OnComponentEndOverlap` _asbp_destructible))))

(event `self.Sphere1.OnComponentEndOverlap`
  (params (OverlappedComponent :type "PrimitiveComponent Object Reference") (OtherActor :type "Actor Object Reference") (OtherComp :type "PrimitiveComponent Object Reference") (OtherBodyIndex :type Integer))
  (bind _asbp_destructible (cast `/Game/Trash/BP_Destructible` OtherActor))
  (`self.Colliding`))

(fn `UserConstructionScript`)
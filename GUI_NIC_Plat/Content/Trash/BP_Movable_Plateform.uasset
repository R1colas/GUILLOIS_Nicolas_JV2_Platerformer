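; BP_Movable_Plateform is a platform actor set up to move through an InterpToMovement component.
; The construction script adds relative control points at the origin and MoveTo, but only when CanMove is true at construction.
; BeginPlay clears CanMove, and Box overlap sets it for BP_ThirdPersonCharacter, storing the character, or clears it for other actors.
; No runtime logic reads the flag, so overlaps do not trigger movement here.
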(event `self.ReceiveBeginPlay`
  (set `self.Can Move` false))

(event `self.Box.OnComponentBeginOverlap`
  (params (OverlappedComponent :type "PrimitiveComponent Object Reference") (OtherActor :type "Actor Object Reference") (OtherComp :type "PrimitiveComponent Object Reference") (OtherBodyIndex :type Integer) (bFromSweep :type Boolean) (SweepResult :type "HitResult Structure (by ref)"))
  (bind _asbp_third_person_character (cast `/Game/Blueprints/BP_ThirdPersonCharacter` OtherActor)
    (:`then`
      (set `self.As BP Third Person Character_0` _asbp_third_person_character)
      (set `self.Can Move` true))
    (:`CastFailed`
      (set `self.Can Move` false))))

(fn `UserConstructionScript`
  (if (`self.Can Move`)
    (`InterpToMovementComponent.AddControlPointPosition` (`self.InterpToMovement`) (0.0 0.0 0.0) true)
    (`InterpToMovementComponent.AddControlPointPosition` (`self.InterpToMovement`) (`self.Move To`) true)))